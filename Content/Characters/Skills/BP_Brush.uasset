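; BP_Brush is a brush skill that fires first-person projectiles, though its Firing event is currently empty.
; SpawnProjectile spawns BP_FirstPersonProjectile at the mesh's Ammo socket, offset and aimed by camera rotation, and calls a sound at that point.
; A disconnected automatic-fire loop, gated by a short delay and noted for rework, holds the only SpawnProjectile call in this file.
; An alternative spawn from the PaintSpawn socket is also unwired.
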(event `Firing`
  (params (Toggle :type Boolean)))

(fn `SpawnProjectile`
  (bind _returnvalue (`PlayerCameraManager.GetCameraRotation` (`GameplayStatics.GetPlayerCameraManager` 0)))
  (bind _returnvalue_2 (+ (`SceneComponent.GetSocketLocation` (`self.SkeletalMesh`) "Ammo") (`KismetMathLibrary.GreaterGreater_VectorRotator` (`self.Projectile Offset`) _returnvalue)))
  (`|SpawnActorFromClass` "/Game/Z_Migrated/Blueprints/BP_FirstPersonProjectile.BP_FirstPersonProjectile_C" (`KismetMathLibrary.MakeTransform` _returnvalue_2 _returnvalue) "Undefined" "OverrideRootScale" null null)
  (`GameplayStatics.PlaySoundAtLocation` null _returnvalue_2 (struct) 1.0 1.0 0.0 null null null null))

(fn `UserConstructionScript`)