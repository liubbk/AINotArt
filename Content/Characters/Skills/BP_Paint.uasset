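; BP_Paint is a paint skill actor that bursts on impact.
; When its Sphere component registers a hit, it spawns the NS_Paint system at the hit location and destroys itself.
; ApplyDamage runs on BeginPlay with no target shown, rather than on impact.
; The old firing logic (delayed collision change, physics impulse) is disconnected, and the generic Hit event is empty.
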(event `self.ReceiveHit`
  (params (MyComp :type "PrimitiveComponent Object Reference") (Other :type "Actor Object Reference") (OtherComp :type "PrimitiveComponent Object Reference") (bSelfMoved :type Boolean) (HitLocation :type "Vector Structure") (HitNormal :type "Vector Structure") (NormalImpulse :type "Vector Structure") (Hit :type "HitResult Structure (by ref)"))
  ;[1 1 1] Old: firing system
)

(event `self.ReceiveBeginPlay`
  (`GameplayStatics.ApplyDamage` null 10.0))

(event `self.Sphere.OnComponentHit`
  (params (HitComponent :type "PrimitiveComponent Object Reference") (OtherActor :type "Actor Object Reference") (OtherComp :type "PrimitiveComponent Object Reference") (NormalImpulse :type "Vector Structure") (Hit :type "HitResult Structure (by ref)"))
  ;[1 1 1] Why isnt working
  (`NiagaraFunctionLibrary.SpawnSystemAtLocation` "/Game/Characters/Skills/NS_Paint.NS_Paint" Hit_Location)
  (`self.K2_DestroyActor`))

(fn `UserConstructionScript`)