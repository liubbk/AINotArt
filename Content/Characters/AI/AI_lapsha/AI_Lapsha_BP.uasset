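; Lapsha enemy AI actor that bites the player character on contact and dies when its health runs out.
; Overlapping its sphere with BP_ThirdPersonCharacter starts the bite montage and applies fixed damage.
; Incoming damage lowers its own LapshaHealth variable, destroying the actor immediately at zero.
; Separately, AI_Health_Component events print health changes and, on depletion, trigger a death montage and delayed destruction.
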(event `self.ReceiveAnyDamage`
  (params (Damage :type "Float (single-precision)") (DamageType :type "DamageType Object Reference") (InstigatedBy :type "Controller Object Reference") (DamageCauser :type "Actor Object Reference"))
  (set `self.Lapsha_Health` (- (`self.Lapsha_Health`) Damage))
  (if (<= (`self.Lapsha_Health`) 0.0)
    (`self.K2_DestroyActor`)))

(event `self.Sphere.OnComponentBeginOverlap`
  (params (OverlappedComponent :type "PrimitiveComponent Object Reference") (OtherActor :type "Actor Object Reference") (OtherComp :type "PrimitiveComponent Object Reference") (OtherBodyIndex :type Integer) (bFromSweep :type Boolean) (SweepResult :type "HitResult Structure (by ref)"))
  (bind _asbp_third_person_character (cast `/Game/ThirdPerson/Blueprints/BP_ThirdPersonCharacter` OtherActor))
  (bind _output_get (set `self.CharRef` _asbp_third_person_character))
  (if (== _output_get OtherActor)
    (`|PlayMontage` (`self.Mesh`) "/Game/Characters/AI/AI_ModelsAnimations/FirstLevelEnemies/Lapsha/Animations/Lapshakusaet_Montage.Lapshakusaet_Montage"
      (:`then`
        (`GameplayStatics.ApplyDamage` _asbp_third_person_character 10.0)))))

(event `self.AI_Health_Component.AI_OnHealthChanged`
  (params (NewHealth :type "Float (double-precision)"))
  (`KismetSystemLibrary.PrintString` (`KismetStringLibrary.Concat_StrStr` "EnemyHealth: " (`KismetStringLibrary.Conv_DoubleToString` NewHealth)) true true (struct :`R` 1.0 :`G` 0.148011 :`A` 1.0) 2.0 "AIHealth"))

(event `self.AI_Health_Component.AI_OnHealthDepleted`
  (`KismetSystemLibrary.PrintString` "Enemy Died" true true (struct :`R` 1.0 :`G` 0.192669 :`A` 1.0))
  (`|PlayMontage` null "/Game/Characters/AI/AI_ModelsAnimations/FirstLevelEnemies/Lapsha/Animations/lapshaumerla_Montage.lapshaumerla_Montage"
    (:`then`
      (`KismetSystemLibrary.Delay` 2.0)
      (`self.K2_DestroyActor`))))

(fn `UserConstructionScript`)