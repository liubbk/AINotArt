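; AI_01_BP is a parent AI actor, per its folder, with a prototype melee-range check for attacking the player.
; Its AttackPlayer event runs a sphere trace for Pawn objects a short distance along the actor's forward vector, with debug drawing enabled.
; A hit that casts to BP_ThirdPersonCharacter only prints a debug message; no damage or animation is applied.
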(event `AttackPlayer`
  (bind _returnvalue (`self.K2_GetActorLocation`))
  (bind (_outhit _returnvalue_2) (`KismetSystemLibrary.SphereTraceSingleForObjects` :`Start` _returnvalue :`End` (+ (* (`KismetMathLibrary.GetForwardVector` (`self.K2_GetActorRotation`)) 250.0) _returnvalue) :`Radius` 120.0 :`ObjectTypes` (`|MakeArray` "ObjectTypeQuery3" :!type "EObjectTypeQuery Enum") :`DrawDebugType` "ForDuration"))
  (if _returnvalue_2
    (cast `/Game/ThirdPerson/Blueprints/BP_ThirdPersonCharacter` (`.HitActor` (`GameplayStatics.BreakHitResult` _outhit)))
    (`KismetSystemLibrary.PrintString` "Attacking")))

(fn `UserConstructionScript`)