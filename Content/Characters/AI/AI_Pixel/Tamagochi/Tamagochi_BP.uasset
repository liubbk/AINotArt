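; Tamagochi AI character shown as a flipbook sprite that turns to face the third-person player.
; A short-delay recursive loop polls until the player is within range, then a second loop continually interpolates yaw toward them.
; The facing loop never rechecks distance, so it keeps running once triggered.
; Tick switches the sprite between walk while moving and punch while stationary.
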(event `self.ReceiveTick`
  (params (DeltaSeconds :type "Float (single-precision)"))
  (`self.UpdateAnimation`))

(event `self.ReceiveBeginPlay`
  ;[1 1 1] Main
  (bind _asbp_third_person_character (cast `/Game/ThirdPerson/Blueprints/BP_ThirdPersonCharacter` (`GameplayStatics.GetPlayerCharacter` 0)))
  (set `self.CharREF` _asbp_third_person_character)
  (`self.ShouldRotate Event`))

(event `FacePlayer Event`
  (bind (_returnvalue_roll _returnvalue_pitch _returnvalue_yaw) (`KismetMathLibrary.BreakRotator` (`KismetMathLibrary.RInterpTo` (`self.K2_GetActorRotation`) (`KismetMathLibrary.FindLookAtRotation` (`self.K2_GetActorLocation`) (`self.K2_GetActorLocation` (`self.CharREF`))) (`GameplayStatics.GetWorldDeltaSeconds`) 50.0)))
  ;[0.8009 0.562 1] Always Face Player
  (if (`self.ShouldRotate?`)
    (`self.K2_SetActorRotation` (`KismetMathLibrary.MakeRotator` 0.0 0.0 _returnvalue_yaw))
    (`KismetSystemLibrary.Delay` 1e-05)
    (`self.FacePlayer Event`)
    (else
      (`self.ShouldRotate Event`))))

(event `ShouldRotate Event`
  ;[0.5736 0.5619 1] Check Rotate
  (if (<= (`self.GetDistanceTo` (`self.CharREF`) null) 1000.0)
    (set `self.ShouldRotate?` true)
    (`self.FacePlayer Event`)
    (else
      (set `self.ShouldRotate?` false)
      (`KismetSystemLibrary.Delay` 0.0001)
      (`self.ShouldRotate Event`))))

(event `UpdateAnimation`
  (`PaperFlipbookComponent.SetFlipbook` (`self.Sprite`) (select `bool` (> (`KismetMathLibrary.VSize` (`MovementComponent.Velocity` (`self.CharacterMovement`))) 0.0) :`false` "/Game/Characters/AI/AI_Pixel/Tamagochi/Sprites/SpriteBase/Punch/Tamagochi_Punch_FB.Tamagochi_Punch_FB" :`true` "/Game/Characters/AI/AI_Pixel/Tamagochi/Sprites/Tamagochi_Walk_FB.Tamagochi_Walk_FB" :!type "PaperFlipbook Object Reference")))

(fn `UserConstructionScript`)