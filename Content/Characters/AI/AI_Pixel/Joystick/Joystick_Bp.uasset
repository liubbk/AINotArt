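; Joystick is a flipbook-sprite AI enemy that turns to face the player and damages them on touch.
; Delay-based event loops poll the player's distance and, within range, smoothly yaw the actor toward them, billboard-style.
; Tick picks the walking or punch flipbook based on whether the character has velocity.
; Overlapping its sphere applies damage to the third-person character, independent of the current animation.
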(event `self.ReceiveTick`
  (params (DeltaSeconds :type "Float (single-precision)"))
  (`self.UpdAnim`))

(event `self.ReceiveBeginPlay`
  ;[1 1 1] Main
  (bind _asbp_third_person_character (cast `/Game/ThirdPerson/Blueprints/BP_ThirdPersonCharacter` (`GameplayStatics.GetPlayerCharacter` 0)))
  (set `self.CharREF` _asbp_third_person_character)
  (`self.ShouldRotate Event 3`))

(event `FacePlayer Event 3`
  (bind (_returnvalue_roll _returnvalue_pitch _returnvalue_yaw) (`KismetMathLibrary.BreakRotator` (`KismetMathLibrary.RInterpTo` (`self.K2_GetActorRotation`) (`KismetMathLibrary.FindLookAtRotation` (`self.K2_GetActorLocation`) (`self.K2_GetActorLocation` (`self.CharREF`))) (`GameplayStatics.GetWorldDeltaSeconds`) 50.0)))
  ;[0.8009 0.562 1] Always Face Player
  (if (`self.ShouldRotate?`)
    (`self.K2_SetActorRotation` (`KismetMathLibrary.MakeRotator` 0.0 0.0 _returnvalue_yaw))
    (`KismetSystemLibrary.Delay` 1e-05)
    (`self.FacePlayer Event 3`)
    (else
      (`self.ShouldRotate Event 3`))))

(event `ShouldRotate Event 3`
  ;[0.5736 0.5619 1] Check Rotate
  (if (<= (`self.GetDistanceTo` (`self.CharREF`) null) 1000.0)
    (set `self.ShouldRotate?` true)
    (`self.FacePlayer Event 3`)
    (else
      (set `self.ShouldRotate?` false)
      (`KismetSystemLibrary.Delay` 0.0001)
      (`self.ShouldRotate Event 3`))))

(event `UpdAnim`
  (`PaperFlipbookComponent.SetFlipbook` (`self.Sprite`) (select `bool` (> (`KismetMathLibrary.VSize` (`MovementComponent.Velocity` (`self.CharacterMovement`))) 0.0) :`false` "/Game/Characters/AI/AI_Pixel/Joystick/Sprites/Joistick_Punch.Joistick_Punch" :`true` "/Game/Characters/AI/AI_Pixel/Joystick/Sprites/Joistick_Walking_FB.Joistick_Walking_FB" :!type "PaperFlipbook Object Reference")))

(event `self.Sphere.OnComponentBeginOverlap`
  (params (OverlappedComponent :type "PrimitiveComponent Object Reference") (OtherActor :type "Actor Object Reference") (OtherComp :type "PrimitiveComponent Object Reference") (OtherBodyIndex :type Integer) (bFromSweep :type Boolean) (SweepResult :type "HitResult Structure (by ref)"))
  (bind _asbp_third_person_character (cast `/Game/ThirdPerson/Blueprints/BP_ThirdPersonCharacter` OtherActor))
  (if (== _asbp_third_person_character OtherActor)
    (`GameplayStatics.ApplyDamage` _asbp_third_person_character 10.0)))

(fn `FacePlayer Event`)

(fn `ShouldRotate Event`)

(fn `UserConstructionScript`)