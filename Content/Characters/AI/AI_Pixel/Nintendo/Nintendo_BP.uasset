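; Nintendo pixel AI Blueprint that turns on its yaw axis to face the third-person player character once the player comes within range.
; BeginPlay caches the player and starts a short-Delay polling loop that checks distance.
; Entering range starts a second Delay-driven loop that interpolates toward the look-at yaw, without Tick.
; That loop never rechecks distance, so facing continues after the player moves away.
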(event `self.ReceiveBeginPlay`
  ;[1 1 1] Main
  (bind _asbp_third_person_character (cast `/Game/ThirdPerson/Blueprints/BP_ThirdPersonCharacter` (`GameplayStatics.GetPlayerCharacter` 0)))
  (set `self.CharREF` _asbp_third_person_character)
  (`self.ShouldRotate Event 2`))

(event `FacePlayer Event 2`
  (bind (_returnvalue_roll _returnvalue_pitch _returnvalue_yaw) (`KismetMathLibrary.BreakRotator` (`KismetMathLibrary.RInterpTo` (`self.K2_GetActorRotation`) (`KismetMathLibrary.FindLookAtRotation` (`self.K2_GetActorLocation`) (`self.K2_GetActorLocation` (`self.CharREF`))) (`GameplayStatics.GetWorldDeltaSeconds`) 50.0)))
  ;[0.8009 0.562 1] Always Face Player
  (if (`self.ShouldRotate?`)
    (`self.K2_SetActorRotation` (`KismetMathLibrary.MakeRotator` 0.0 0.0 _returnvalue_yaw))
    (`KismetSystemLibrary.Delay` 1e-05)
    (`self.FacePlayer Event 2`)
    (else
      (`self.ShouldRotate Event 2`))))

(event `ShouldRotate Event 2`
  ;[0.5736 0.5619 1] Check Rotate
  (if (<= (`self.GetDistanceTo` (`self.CharREF`) null) 1000.0)
    (set `self.ShouldRotate?` true)
    (`self.FacePlayer Event 2`)
    (else
      (set `self.ShouldRotate?` false)
      (`KismetSystemLibrary.Delay` 0.0001)
      (`self.ShouldRotate Event 2`))))

(fn `FacePlayer Event`)

(fn `UserConstructionScript`)