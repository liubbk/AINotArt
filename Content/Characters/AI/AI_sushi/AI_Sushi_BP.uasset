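; AI_Sushi_BP is a sushi AI character that throws bomb projectiles and can be destroyed by damage.
; ShootProjectile checks that the player is BP_ThirdPersonCharacter, waits briefly, spawns Projectile_02_BP at ProjectileSpawn, then plays a sped-up shooting montage.
; AnyDamage subtracts from SushiHealth and, as written, plays the death montage and destroys the actor while health is still zero or above, rather than when depleted.
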(event `ShootProjectile`
  (bind _projectilespawn (`self.ProjectileSpawn`))
  ;[1 0.3407 0.3008] ThrowBombs
  (cast `/Game/ThirdPerson/Blueprints/BP_ThirdPersonCharacter` (`GameplayStatics.GetPlayerCharacter` 0))
  (`KismetSystemLibrary.Delay` 1.0)
  (`|SpawnActorFromClass` "/Game/Characters/AI/AI_sushi/Projectiles/Projectile_02_BP.Projectile_02_BP_C" (`KismetMathLibrary.MakeTransform` (`SceneComponent.K2_GetComponentLocation` _projectilespawn) (`SceneComponent.K2_GetComponentRotation` _projectilespawn)) "Undefined" "OverrideRootScale" null null)
  (`|PlayMontage` null "/Game/Characters/AI/AI_ModelsAnimations/FirstLevelEnemies/Sushi/Animations/Shooting_AM.Shooting_AM" 5.0))

(event `self.ReceiveAnyDamage`
  (params (Damage :type "Float (single-precision)") (DamageType :type "DamageType Object Reference") (InstigatedBy :type "Controller Object Reference") (DamageCauser :type "Actor Object Reference"))
  (set `self.SushiHealth` (- (`self.SushiHealth`) Damage))
  (if (>= (`self.SushiHealth`) 0.0)
    (`self.PlayAnimMontage` "/Game/Characters/AI/AI_ModelsAnimations/FirstLevelEnemies/Sushi/Animations/Death_Sushi_AM.Death_Sushi_AM")
    (`KismetSystemLibrary.Delay` 1.0)
    (`self.K2_DestroyActor`)))

(fn `UserConstructionScript`)